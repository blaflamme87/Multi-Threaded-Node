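; BP_PrimeCalculator is an actor that runs a heavy prime search when a pawn overlaps its Box, comparing threaded and blocking execution.
; ShouldUseMultiThreaded selects whether FindPrimes runs inside a MultiThreadedNode or directly on the game thread, with "FINISHED" printed afterward.
; FindPrimes uses brute-force trial division to reach 2000 primes, logging every tenth.
; Its counters are never reset between overlaps.
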(event `self.Box.OnComponentBeginOverlap`
  (params (OverlappedComponent :type "PrimitiveComponent Object Reference") (OtherActor :type "Actor Object Reference") (OtherComp :type "PrimitiveComponent Object Reference") (OtherBodyIndex :type Integer) (bFromSweep :type Boolean) (SweepResult :type "HitResult Structure (by ref)"))
  (cast `Pawn` OtherActor)
  (if (`self.ShouldUseMultiThreaded`)
    (`AsyncActionNode.MultiThreadedNode`
      (:`MultiThreadedWork`
        (`self.FindPrimes` 2000))
      (:`FinishedWork`
        (`KismetSystemLibrary.PrintString` "FINISHED")))
    (else
      (`self.FindPrimes` 2000)
      (`KismetSystemLibrary.PrintString` "FINISHED"))))

(fn `FindPrimes`
  (params (NumPrimesToFind :type Integer))
  (locals (IsPrime :type Boolean) (PrimesFound :type Integer) (CurrentTestNumber :type Integer))
  (while (< (`local.PrimesFound`) NumPrimesToFind)
    (set `local.IsPrime` true)
    (for _index (range 2 (+ (/ (`local.CurrentTestNumber`) 2) 1))
      (if (== (mod (`local.CurrentTestNumber`) _index) 0)
        (set `local.IsPrime` false)
        (break)))
    (`|ExecutionSequence`
      (:`then_0`
        (if (`local.IsPrime`)
          (`/Engine/EditorBlueprintResources/StandardMacros.IncrementInt` (`local.PrimesFound`)
            (:`  `
              (if (== (mod (`local.PrimesFound`) 10) 0)
                (`KismetSystemLibrary.PrintString` (`KismetStringLibrary.Concat_StrStr` "Primes found: " (`KismetStringLibrary.Conv_IntToString` (`local.PrimesFound`))) false))))))
      (:`then_1`
        (`/Engine/EditorBlueprintResources/StandardMacros.IncrementInt` (`local.CurrentTestNumber`))))))

(fn `UserConstructionScript`)